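; TestActor is a test actor set up to move along the spline of a Track actor.
; BeginPlay stores the first Track found in the level.
; An unconnected timeline holds the movement, which derives distance from Speed and game time and sets the actor's location from the spline's local-space point.
; Nothing triggers that timeline, so the actor does not move as the graph stands.
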(event Collision|EventActorBeginOverlap
  (params (OtherActor :type Actor%20Object%20Reference)))

(event EventTick
  (params (DeltaSeconds :type Float%20%28single-precision%29)))

(event EventBeginPlay
  (bind _outactors (Actor|GetAllActorsOfClass "/Game/Blueprints/Track.Track_C"))
  (Variables|Default|SetTrack (Utilities|Array|Get(acopy) _outactors)))

(fn ConstructionScript)